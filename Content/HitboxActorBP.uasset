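; Hitbox actor for a fighting game that displays a proximity, strike or hurtbox volume and damages the player character on contact.
; SpawnHitbox picks a debug material by hitbox type, moves the display component to the hitbox location and makes it visible.
; It then runs a one-time overlap check against player character 0, casting it to FightingGameCharacter and applying the hitbox damage.
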(event `SpawnHitbox`
  (switch `EHitboxEnum` (`self.hitboxType`)
    (:`HB_PROXIMITY`
      (`PrimitiveComponent.SetMaterial` (`self.HitboxDisplay`) 0 "/Game/Art/Materials/Hitboxes/M_ProximityHitBox.M_ProximityHitBox"))
    (:`HB_STRIKE`
      (`PrimitiveComponent.SetMaterial` (`self.HitboxDisplay`) 0 "/Game/Art/Materials/Hitboxes/M_StrikeHitBox.M_StrikeHitBox"))
    (:`HB_HURTBOX`
      (`PrimitiveComponent.SetMaterial` (`self.HitboxDisplay`) 0 "/Game/Art/Materials/Hitboxes/M_HurtBox.M_HurtBox")))
  (`SceneComponent.K2_SetWorldLocation` (`self.HitboxDisplay`) (`self.hitboxLocation`) false false)
  (`SceneComponent.SetVisibility` (`self.HitboxDisplay`) true false)
  (`self.CheckCollision`))

(event `CheckCollision`
  (bind _returnvalue (`GameplayStatics.GetPlayerCharacter` 0))
  (if (`self.IsOverlappingActor` _returnvalue)
    (bind _asfighting_game_character (cast `FightingGameCharacter` _returnvalue))
    (`FightingGameCharacter.TakeDamage2` _asfighting_game_character (`self.hitboxDamage`))))

(fn `spawnHitBox1`)

(fn `UserConstructionScript`)